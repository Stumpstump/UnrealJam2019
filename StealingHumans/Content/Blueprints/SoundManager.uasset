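; SoundManager is an actor that plays vocal reactions when a human character is tapped.
; PlayHumanTapSound takes a gender flag and a human type index, then refills a shared sound array with that combination's pair of clips, covering adult, elderly, kid and one other type.
; All branches converge on a single node that plays a random entry from the array as non-spatial 2D audio.
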(event `PlayHumanTapSound`
  (params (isMale :type Boolean) (humanType :type Integer))
  (bind _soundarray (`self.soundArray`))
  (bind _soundarray_2 (`self.soundArray`))
  (`KismetArrayLibrary.Array_Clear` (`self.soundArray`))
  (if isMale
    (switch `int` humanType
      (:`0`
        (`KismetArrayLibrary.Array_Add` _soundarray "/Game/Audio/Man-VOs/Man/M_Adult_Hmm_2.M_Adult_Hmm_2")
        (`KismetArrayLibrary.Array_Add` _soundarray "/Game/Audio/Man-VOs/Man/M_Adult_Hmm_1.M_Adult_Hmm_1"))
      (:`1`
        (`KismetArrayLibrary.Array_Add` _soundarray "/Game/Audio/Man-VOs/Man/M_Elderly_Oh_1.M_Elderly_Oh_1")
        (`KismetArrayLibrary.Array_Add` _soundarray "/Game/Audio/Man-VOs/Man/M_Elderly_Oh_2.M_Elderly_Oh_2"))
      (:`2`
        (`KismetArrayLibrary.Array_Add` _soundarray "/Game/Audio/NicsAudio/VocalUhh.VocalUhh")
        (`KismetArrayLibrary.Array_Add` _soundarray "/Game/Audio/NicsAudio/Vocalwhat.Vocalwhat"))
      (:`3`
        (`KismetArrayLibrary.Array_Add` _soundarray "/Game/Audio/Man-VOs/Man/M_Kid_Hmm_1.M_Kid_Hmm_1")
        (`KismetArrayLibrary.Array_Add` _soundarray "/Game/Audio/Man-VOs/Man/M_Kid_Hmm_2.M_Kid_Hmm_2")))
    (else
      (switch `int` humanType
        (:`0`
          (`KismetArrayLibrary.Array_Add` _soundarray "/Game/Audio/Woman-VOs/Woman/W_Adult_Hmm_1.W_Adult_Hmm_1")
          (`KismetArrayLibrary.Array_Add` _soundarray "/Game/Audio/Woman-VOs/Woman/W_Adult_Hmm_2.W_Adult_Hmm_2"))
        (:`1`
          (`KismetArrayLibrary.Array_Add` _soundarray "/Game/Audio/Woman-VOs/Woman/W_Elderly_Hmm_1.W_Elderly_Hmm_1")
          (`KismetArrayLibrary.Array_Add` _soundarray "/Game/Audio/Woman-VOs/Woman/W_Elderly_Hmm_2.W_Elderly_Hmm_2"))
        (:`2`
          (`KismetArrayLibrary.Array_Add` _soundarray "/Game/Audio/NicsAudio/VocalGasp.VocalGasp")
          (`KismetArrayLibrary.Array_Add` _soundarray "/Game/Audio/NicsAudio/VocalGasp.VocalGasp"))
        (:`3`
          (`KismetArrayLibrary.Array_Add` _soundarray "/Game/Audio/Woman-VOs/Woman/W_Kid_Hmm_1.W_Kid_Hmm_1")
          (`KismetArrayLibrary.Array_Add` _soundarray "/Game/Audio/Woman-VOs/Woman/W_Kid_Hmm_2.W_Kid_Hmm_2")))))
  (`GameplayStatics.PlaySound2D` (`|GetArrayItem` _soundarray_2 (`KismetMathLibrary.RandomIntegerInRange` 0 (`KismetArrayLibrary.Array_LastIndex` _soundarray_2))) 1.0 1.0 0.0 null null))

(event `CustomEvent_0`)

(fn `UserConstructionScript`)