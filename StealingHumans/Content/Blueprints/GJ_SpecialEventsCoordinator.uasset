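; Coordinator actor that runs three timed random special events once started: find item, dragging bonus and chase object.
; Each event loops independently on timers, rolling a percent chance after a delay, then running for a set duration while Tick tracks its progress.
; Find and chase events spawn actors at random spawn points and award Alien or Reptile points through GJ_GameMode on success.
; Dragging temporarily changes the game mode's HumanPointMultiplier.
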(event `self.ReceiveBeginPlay`)

(event `StartSpecialEvents`
  (bind _outactors (`GameplayStatics.GetAllActorsOfClass` "/Game/Blueprints/SpawnPOints/FindItemSpawnPoint.FindItemSpawnPoint_C"))
  (set `self.FindItemSpawnPoints` _outactors)
  (`self.FindItemRoutine`)
  (`self.DraggingRoutine`)
  (bind _outactors_2 (`GameplayStatics.GetAllActorsOfClass` "/Game/Blueprints/SpawnPOints/ChaseObjectSpawnPoint.ChaseObjectSpawnPoint_C"))
  (set `self.CatChaseSpawnPoints` _outactors_2)
  (`self.CatChaseRoutine`))

(event `self.ReceiveTick`
  (params (DeltaSeconds :type "Float (single-precision)"))
  (set `self.FindItemTimeLerp` (/ (`KismetSystemLibrary.K2_GetTimerElapsedTimeHandle` (stale `TryFindItem` _returnvalue)) (`KismetMathLibrary.Conv_IntToDouble` (`self.FindItemEventTime`))))
  (set `self.DraggingTimeLerp` (/ (`KismetSystemLibrary.K2_GetTimerElapsedTimeHandle` (stale `TryDragging` _returnvalue)) (`KismetMathLibrary.Conv_IntToDouble` (`self.DraggingEventTime`))))
  (set `self.CatChaseTimeLerp` (/ (`KismetSystemLibrary.K2_GetTimerElapsedTimeHandle` (stale `TryCatChase` _returnvalue)) (`KismetMathLibrary.Conv_IntToDouble` (`self.CatChaseEventTime`)))))

(event `FindItemRoutine`
  ;[1 1 1] Find Item Event
  (`KismetSystemLibrary.K2_SetTimerDelegate` (delegate `TryFindItem`) (`KismetMathLibrary.Conv_IntToDouble` (`self.FindItemEventDelay`))))

(event `TryFindItem`
  ;[1 1 1] Find Item Event
  (if (< (`KismetMathLibrary.RandomIntegerInRange` 0 99) (`self.FindItemPercentChance`))
    (`self.SpawnFindItem`)
    (bind _returnvalue (`KismetSystemLibrary.K2_SetTimerDelegate` (delegate `EndFindItem`) (`KismetMathLibrary.Conv_IntToDouble` (`self.FindItemEventTime`))))
    (else
      (`self.FindItemRoutine`))))

(event `EndFindItem`
  (bind _finditem (`self.FindItem`))
  ;[1 1 1] Find Item Event
  (`/Engine/EditorBlueprintResources/StandardMacros.IsValid` _finditem
    (:`Is Valid`
      (`self.K2_DestroyActor` _finditem)
      (set `self.FindItem` null)
      (`self.FindItemRoutine`))))

(event `ItemFound`
  (params (isAlien :type Boolean))
  (bind _finditempointvalue (`self.FindItemPointValue`))
  ;[1 1 1] Find Item Event
  (bind _asgj_game_mode (cast `/Game/Blueprints/GJ_GameMode` (`GameplayStatics.GetGameMode`)))
  (if isAlien
    (`/Game/Blueprints/GJ_GameMode.AddAlienPoints` _asgj_game_mode _finditempointvalue false)
    (else
      (`/Game/Blueprints/GJ_GameMode.AddReptilePoints` _asgj_game_mode _finditempointvalue false)))
  (`KismetSystemLibrary.K2_ClearAndInvalidateTimerHandle` (stale `TryFindItem` _returnvalue))
  (`self.EndFindItem`))

(event `DraggingRoutine`
  ;[1 1 1] Dragging Event
  (`KismetSystemLibrary.K2_SetTimerDelegate` (delegate `TryDragging`) (`KismetMathLibrary.Conv_IntToDouble` (`self.DraggingEventDelay`))))

(event `TryDragging`
  ;[1 1 1] Dragging Event
  (if (< (`KismetMathLibrary.RandomIntegerInRange` 0 99) (`self.DraggingPercentChance`))
    (`self.DraggingMode` true)
    (bind _returnvalue (`KismetSystemLibrary.K2_SetTimerDelegate` (delegate `EndDragging`) (`KismetMathLibrary.Conv_IntToDouble` (`self.DraggingEventTime`))))
    (else
      (`self.DraggingRoutine`))))

(event `EndDragging`
  ;[1 1 1] Dragging Event
  (`self.DraggingMode` false)
  (`self.DraggingRoutine`))

(event `CatChaseRoutine`
  ;[1 1 1] Chase Object Event
  (`KismetSystemLibrary.K2_SetTimerDelegate` (delegate `TryCatChase`) (`KismetMathLibrary.Conv_IntToDouble` (`self.CatChaseEventDelay`))))

(event `TryCatChase`
  ;[1 1 1] Chase Object Event
  (if (< (`KismetMathLibrary.RandomIntegerInRange` 0 99) (`self.CatChasePercentChance`))
    (`self.SpawnChaseObject`)
    (bind _returnvalue (`KismetSystemLibrary.K2_SetTimerDelegate` (delegate `EndCatChase`) (`KismetMathLibrary.Conv_IntToDouble` (`self.CatChaseEventTime`))))
    (else
      (`self.CatChaseRoutine`))))

(event `EndCatChase`
  (bind _chaseobject (`self.ChaseObject`))
  ;[1 1 1] Chase Object Event
  (`/Engine/EditorBlueprintResources/StandardMacros.IsValid` _chaseobject
    (:`Is Valid`
      (`self.K2_DestroyActor` _chaseobject)
      (set `self.ChaseObject` null))
    (:`Is Not Valid`
      _))
  (`self.CatChaseRoutine`))

(event `ChaseCaught`
  (params (isAlien :type Boolean))
  (bind _catchasepointvalue (`self.CatChasePointValue`))
  ;[1 1 1] Chase Object Event
  (bind _asgj_game_mode (cast `/Game/Blueprints/GJ_GameMode` (`GameplayStatics.GetGameMode`)))
  (if isAlien
    (`/Game/Blueprints/GJ_GameMode.AddAlienPoints` _asgj_game_mode _catchasepointvalue false)
    (else
      (`/Game/Blueprints/GJ_GameMode.AddReptilePoints` _asgj_game_mode _catchasepointvalue false)))
  (`KismetSystemLibrary.K2_ClearAndInvalidateTimerHandle` (stale `TryCatChase` _returnvalue))
  (`self.EndCatChase`))

(fn `DraggingMode`
  (params (modeOn :type Boolean))
  (bind _asgj_game_mode (cast `/Game/Blueprints/GJ_GameMode` (`GameplayStatics.GetGameMode`)))
  (if modeOn
    (set `/Game/Blueprints/GJ_GameMode.HumanPointMultiplier` (`self.DraggingPointMultiplier`) _asgj_game_mode)
    (else
      (set `/Game/Blueprints/GJ_GameMode.HumanPointMultiplier` 1.0 _asgj_game_mode))))

(fn `SpawnChaseObject`
  (bind _catchasespawnpoints (`self.CatChaseSpawnPoints`))
  (bind _returnvalue (`|SpawnActorFromClass` "/Game/Blueprints/ChaseObject.ChaseObject_C" (`self.GetTransform` (`|GetArrayItem` _catchasespawnpoints (`KismetMathLibrary.RandomIntegerInRange` 0 (`KismetArrayLibrary.Array_LastIndex` _catchasespawnpoints)))) "Undefined" "OverrideRootScale" null null))
  (set `self.ChaseObject` _returnvalue))

(fn `SpawnFindItem`
  (locals (FindItemClass :type "/Game/Blueprints/FindItem Class Reference"))
  (bind _finditemspawnpoints (`self.FindItemSpawnPoints`))
  (switch `int` (`KismetMathLibrary.RandomIntegerInRange` 0 2)
    (:`0`
      (set `local.FindItemClass` "/Game/Blueprints/Find_Rose.Find_Rose_C"))
    (:`1`
      (set `local.FindItemClass` "/Game/Blueprints/Find_IceCream.Find_IceCream_C"))
    (:`2`
      (set `local.FindItemClass` "/Game/Blueprints/Find_Magazine.Find_Magazine_C")))
  (bind _returnvalue (`|SpawnActorFromClass` (`local.FindItemClass`) (`self.GetTransform` (`|GetArrayItem` _finditemspawnpoints (`KismetMathLibrary.RandomIntegerInRange` 0 (`KismetArrayLibrary.Array_LastIndex` _finditemspawnpoints)))) "Undefined" "OverrideRootScale" null null))
  (set `self.FindItem` _returnvalue))

(fn `UserConstructionScript`)