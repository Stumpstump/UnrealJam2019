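; GJ_HUD is the game's HUD class, switching between the main menu, in-game UI and game-over display.
; Show events clear all widgets, lazily create and cache the menu or game UI, then set input mode and cursor visibility to match.
; The end-game event shows the cursor and passes the winner to the existing game UI's GameOver rather than creating a separate widget.
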(event `self.ReceiveBeginPlay`)

(event `ShowMainMenuhud`
  (bind _returnvalue (`GameplayStatics.GetPlayerController` 0))
  (`WidgetLayoutLibrary.RemoveAllWidgets`)
  (`/Engine/EditorBlueprintResources/StandardMacros.IsValid` (`self.m_MainMenu`)
    (:`Is Valid`
      _)
    (:`Is Not Valid`
      (bind _returnvalue_2 (`|CreateWidget` "/Game/Blueprints/Menus/GJ_MainMenu.GJ_MainMenu_C"))
      (set `self.m_MainMenu` _returnvalue_2)))
  (`UserWidget.AddToViewport` (`self.m_MainMenu`) 0)
  (`WidgetBlueprintLibrary.SetInputMode_UIOnlyEx` _returnvalue (`/Game/Blueprints/Menus/GJ_MainMenu.HowToPlayButton` (`self.m_MainMenu`)))
  (set `PlayerController.bShowMouseCursor` true _returnvalue))

(event `ShowGameUIhud`
  (bind _returnvalue (`GameplayStatics.GetPlayerController` 0))
  (`WidgetLayoutLibrary.RemoveAllWidgets`)
  (`/Engine/EditorBlueprintResources/StandardMacros.IsValid` (`self.m_GameUI`)
    (:`Is Valid`
      _)
    (:`Is Not Valid`
      (bind _returnvalue_2 (`|CreateWidget` "/Game/Blueprints/Menus/GJ_GameUI.GJ_GameUI_C"))
      (set `self.m_GameUI` _returnvalue_2)))
  (`UserWidget.AddToViewport` (`self.m_GameUI`) 0)
  (`WidgetBlueprintLibrary.SetInputMode_GameOnly` _returnvalue)
  (set `PlayerController.bShowMouseCursor` false _returnvalue))

(event `ShowEndGameUI`
  (params (winner :type Integer))
  (set `PlayerController.bShowMouseCursor` true (`GameplayStatics.GetPlayerController` 0))
  (`/Game/Blueprints/Menus/GJ_GameUI.GameOver` (`self.m_GameUI`) winner))

(fn `UserConstructionScript`)