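; BasePointer is an indicator actor, parented to a GJ_PlayerCharacter, that marks the direction of that player's base.
; On BeginPlay it caches the parent player and finds either AlienBase_BP or ReptileBase_BP, based on the player's IsAlien flag.
; Every tick it moves itself to an Offset distance from the player along the normalized direction toward that base, changing only location, not rotation.
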(event `self.ReceiveBeginPlay`
  (bind _asgj_player_character (cast `/Game/Blueprints/GJ_PlayerCharacter` (`self.GetParentActor`)))
  (bind _output_get (set `self.dad` _asgj_player_character))
  (if (`/Game/Blueprints/GJ_PlayerCharacter.isAlien` _output_get)
    (bind _returnvalue (`GameplayStatics.GetActorOfClass` "/Game/Blueprints/AlienBase_BP.AlienBase_BP_C"))
    (set `self.myBase` _returnvalue)
    (else
      (bind _returnvalue_2 (`GameplayStatics.GetActorOfClass` "/Game/Blueprints/ReptileBase_BP.ReptileBase_BP_C"))
      (set `self.myBase` _returnvalue_2))))

(event `self.ReceiveTick`
  (params (DeltaSeconds :type "Float (single-precision)"))
  (bind _returnvalue (`self.K2_GetActorLocation` (`self.dad`)))
  (`self.K2_SetActorLocation` (+ (* (`KismetMathLibrary.Normal` (- (`self.K2_GetActorLocation` (`self.myBase`)) _returnvalue)) (`self.offset`)) _returnvalue)))

(fn `UserConstructionScript`)