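; Modular character mesh actor that assembles a human or player look from hair, clothing, head, face and accessory slots.
; Construction master-poses child meshes to MasterMesh and gathers each slot's options, then BeginPlay shows one per slot by index, or randomly, rerolling "NoRandom" tags.
; Slots also switch by tag, and head meshes can hide hair.
; It mirrors parent NPC or player state into CharacterAnimBP and supplies random drag bones; EnableRagdoll is stubbed out.
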(event `self.ReceiveBeginPlay`
  (bind _returnvalue (`self.GetParentActor`))
  (bind _returnvalue_2 (`SkeletalMeshComponent.GetAnimInstance` (`self.Master Mesh`)))
  (`|ExecutionSequence`
    (:`then_0`
      ;[1 1 1] Initialize Slots
      (`self.Set Slot` (`self.HairSets`) (`self.InitialHair`))
      (`self.Set Slot` (`self.ShirtSets`) (`self.InitialShirt`))
      (`self.Set Slot` (`self.PantsSets`) (`self.InitialPants`))
      (`self.Set Slot` (`self.ShoesSets`) (`self.InitialShoes`))
      (`self.Set Slot` (`self.HeadSets`) (`self.InitialHead`))
      (`self.Set Slot` (`self.FaceSets`) (`self.InitialFace`))
      (`self.Set Slot` (`self.AccessorySets`) (`self.InitialAccessory`)))
    (:`then_1`
      ;[1 1 1] Cache Anim
      (set `self.Anim` (cast `/Game/Blueprints/CharacterAnimBP` (`SkeletalMeshComponent.GetAnimInstance` (`self.Master Mesh`)) :!pure true)))
    (:`then_2`
      (bind _asnpc_human (cast `/Game/Blueprints/NPC_Human` _returnvalue)
        (:`then`
          (set `self.MyNPCHuman` _asnpc_human)
          (bind _ascharacter_anim_bp (cast `/Game/Blueprints/CharacterAnimBP` _returnvalue_2))
          (set `self.myAnimBP` _ascharacter_anim_bp))
        (:`CastFailed`
          (bind _asgj_player_character (cast `/Game/Blueprints/GJ_PlayerCharacter` _returnvalue))
          (set `self.MyPlayerCharacter` _asgj_player_character)
          (bind _ascharacter_anim_bp_2 (cast `/Game/Blueprints/CharacterAnimBP` _returnvalue_2))
          (bind _output_get (set `self.myAnimBP` _ascharacter_anim_bp_2))
          (set `/Game/Blueprints/CharacterAnimBP.isAlien` (`/Game/Blueprints/GJ_PlayerCharacter.isAlien` _asgj_player_character) _output_get))))))

(event `self.ReceiveTick`
  (params (DeltaSeconds :type "Float (single-precision)"))
  (bind _myanimbp (`self.myAnimBP`))
  (`/Engine/EditorBlueprintResources/StandardMacros.IsValid` (`self.MyNPCHuman`)
    (:`Is Valid`
      (set `/Game/Blueprints/CharacterAnimBP.isDragged` (`|EnumEquality` (`/Game/Blueprints/NPC_Human.MyState` (`self.MyNPCHuman`)) "NewEnumerator2") _myanimbp)
      (set `/Game/Blueprints/CharacterAnimBP.isTapped` (`|EnumEquality` (`/Game/Blueprints/NPC_Human.MyState` (`self.MyNPCHuman`)) "NewEnumerator1") _myanimbp)
      (set `/Game/Blueprints/CharacterAnimBP.isAlien` false _myanimbp))
    (:`Is Not Valid`
      (`/Engine/EditorBlueprintResources/StandardMacros.IsValid` (`self.MyPlayerCharacter`)
        (:`Is Valid`
          (set `/Game/Blueprints/CharacterAnimBP.isDragging` (`KismetSystemLibrary.IsValid` (`/Game/Blueprints/GJ_PlayerCharacter.DraggedHuman` (`self.MyPlayerCharacter`))) (`self.myAnimBP`)))))))

(fn `Enable Ragdoll`
  (params (`Is Ragdoll` :type Boolean)))

(fn `Get Drag Bone`
  (returns (`Mesh Component` :type "SkinnedMeshComponent Object Reference") (`Drag Bone` :type Name))
  (bind _dragbones (`self.DragBones`))
  (return (`self.Master Mesh`) (select `bool` (> (`KismetArrayLibrary.Array_Length` _dragbones) 0) :`true` (`|GetArrayItem` _dragbones (`KismetMathLibrary.RandomIntegerInRange` 0 (`KismetArrayLibrary.Array_LastIndex` _dragbones))))))

(fn `Init Slot`
  (params (Slot :type "SceneComponent Object Reference (by ref)") (Sets :type "Array of MeshComponent Object Reference (by ref)"))
  (`KismetArrayLibrary.Array_Clear` Sets)
  (for _array_element (`SceneComponent.GetChildrenComponents` Slot false)
    (bind _asmesh_component (cast `MeshComponent` _array_element))
    (`KismetArrayLibrary.Array_Add` Sets _asmesh_component))
  ;[1 1 1] Set first element if available
  (if (> (`KismetArrayLibrary.Array_Length` Sets) 0)
    (`self.Set Slot` Sets)))

(fn `Set Anim Speed`
  (params (Speed :type "Float (double-precision)"))
  (set `/Game/Blueprints/CharacterAnimBP.Speed` Speed (`self.Anim`)))

(fn `Set Slot`
  (params (Sets :type "Array of MeshComponent Object Reference") (Index :type Integer))
  (locals (ValidatedIndex :type Integer) (IsRandom :type Boolean))
  (bind _returnvalue (`KismetArrayLibrary.Array_LastIndex` Sets))
  (bind _returnvalue_2 (== Index -1))
  (set `local.IsRandom` _returnvalue_2)
  (set `local.ValidatedIndex` (select `bool` _returnvalue_2 :`false` (`KismetMathLibrary.Clamp` Index 0 _returnvalue) :`true` (`KismetMathLibrary.RandomIntegerInRange` 0 _returnvalue)) :!label _label)
  (for (_array_element _array_index) Sets
    (`/Engine/EditorBlueprintResources/StandardMacros.IsValid` _array_element
      (:`Is Valid`
        (bind _returnvalue_3 (== _array_index (`local.ValidatedIndex`)))
        (if _returnvalue_3
          (if (or (not (`local.IsRandom`)) (not (`ActorComponent.ComponentHasTag` _array_element "NoRandom")))
            _
            (else
              (goto _label))))
        (`SceneComponent.SetVisibility` _array_element _returnvalue_3 true)
        (if _returnvalue_3
          (`BlueprintMapLibrary.Map_Add` (`self.VisibleMeshes`) (`SceneComponent.GetAttachParent` _array_element) _array_element)))))
  (`self.Update Slot Dependencies`))

(fn `Set Slot By Tag`
  (params (SlotName :type "/Game/Blueprints/Enums/Slot Enum" :default "NewEnumerator0") (SetName :type Name) (`Is Initial` :type Boolean))
  (returns (`Is Success` :type Boolean))
  (locals (FoundSet :type Boolean))
  (bind (_value _returnvalue) (`BlueprintMapLibrary.Map_Find` (`self.Slots`) (`KismetStringLibrary.Conv_StringToName` (`|GetEnumeratorNameAsString` SlotName))))
  (if _returnvalue
    (for (_array_element _array_index) (`SceneComponent.GetChildrenComponents` _value false)
      (bind _returnvalue_2 (`ActorComponent.ComponentHasTag` _array_element SetName))
      (`SceneComponent.SetVisibility` _array_element _returnvalue_2 true)
      (bind _output_get (set `local.FoundSet` (or _returnvalue_2 (`local.FoundSet`))))
      (if (and _output_get (`local.Is Initial`))
        (switch `/Game/Blueprints/Enums/Slot` (`local.SlotName`)
          (:`NewEnumerator0`
            (set `self.InitialHair` _array_index))
          (:`NewEnumerator1`
            (set `self.InitialShirt` _array_index))
          (:`NewEnumerator2`
            (set `self.InitialPants` _array_index))
          (:`NewEnumerator3`
            (set `self.InitialShoes` _array_index))
          (:`NewEnumerator4`
            (set `self.InitialHead` _array_index))
          (:`NewEnumerator5`
            (set `self.InitialFace` _array_index))
          (:`NewEnumerator6`
            (set `self.InitialAccessory` _array_index)))))
    (`self.Update Slot Dependencies`)
    (return (`local.FoundSet`))))

(fn `Update Slot Dependencies`
  (if (`self.HideHairIfHead`)
    (bind _asskeletal_mesh_component (cast `SkeletalMeshComponent` (`BlueprintMapLibrary.Map_Find` (`self.VisibleMeshes`) (`self.SlotHead`))))
    (for _array_element (`self.HairSets`)
      (`SceneComponent.SetVisibility` _array_element (select `bool` (not (`KismetSystemLibrary.IsValid` (`SkinnedMeshComponent.SkeletalMesh` _asskeletal_mesh_component))) :`true` (== _array_element (`BlueprintMapLibrary.Map_Find` (`self.VisibleMeshes`) (`self.SlotHair`)))) true) ; Hide hair if hat visible
    )))

(fn `UserConstructionScript`
  (bind _master_mesh (`self.Master Mesh`))
  (for _array_element (`SceneComponent.GetChildrenComponents` _master_mesh true)
    (bind _asskinned_mesh_component (cast `SkinnedMeshComponent` _array_element))
    (`SkinnedMeshComponent.SetLeaderPoseComponent` _asskinned_mesh_component _master_mesh false))
  (`BlueprintMapLibrary.Map_Clear` (`self.VisibleMeshes`))
  (`self.Init Slot` (`self.SlotHair`) (`self.HairSets`))
  (`self.Init Slot` (`self.SlotShirt`) (`self.ShirtSets`))
  (`self.Init Slot` (`self.SlotPants`) (`self.PantsSets`))
  (`self.Init Slot` (`self.SlotShoes`) (`self.ShoesSets`))
  (`self.Init Slot` (`self.SlotHead`) (`self.HeadSets`))
  (`self.Init Slot` (`self.SlotFace`) (`self.FaceSets`))
  (`self.Init Slot` (`self.SlotAccessory`) (`self.AccessorySets`))
  (for _array_element_2 (`SceneComponent.GetChildrenComponents` (`self.Master Mesh`) false)
    (if (`ActorComponent.ComponentHasTag` _array_element_2 "Slot")
      (for _array_element_3 (`ActorComponent.ComponentTags` _array_element_2)
        (if (and (!= _array_element_3 "Slot") (`KismetStringLibrary.StartsWith` (`KismetStringLibrary.Conv_NameToString` _array_element_3) "Slot"))
          (`BlueprintMapLibrary.Map_Add` (`self.Slots`) _array_element_3 _array_element_2)
          (break))))))