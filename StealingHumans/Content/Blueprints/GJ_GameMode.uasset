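; Game mode for a Reptile versus Alien game, solo or local two-player, where teams score points from humans.
; BeginPlay spawns weighted human types on a shuffled share of spawn points, blends the menu camera and shows the main menu.
; StartGame spawns players at tagged PlayerStarts and starts a countdown, with danger music near the end.
; Timeout or passing PointsToWin calls GameOver, which, if enabled, disables input and shows the winner.
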(event `self.ReceiveBeginPlay`
  (bind _returnvalue (`GameplayStatics.GetPlayerController` 0))
  (bind _menucameratransitiontime (`self.MenuCameraTransitionTime`))
  (`self.SpawnHumans`)
  (if (`self.MusicOn`)
    (bind _returnvalue_2 (`GameplayStatics.SpawnSound2D` "/Game/Audio/Music/Xylocraft_Cue.Xylocraft_Cue" 1.0 1.0 0.0 null))
    (set `self.CurrentMusic` _returnvalue_2))
  ;[1 1 1] MenuCameraTransitions
  (`KismetSystemLibrary.Delay` 0.2)
  (bind _returnvalue_3 (`GameplayStatics.GetActorOfClass` "/Game/Blueprints/MenuCameras_BP.MenuCameras_BP_C"))
  (`/Engine/EditorBlueprintResources/StandardMacros.IsValid` _returnvalue_3
    (:`Is Valid`
      (`PlayerController.SetViewTargetWithBlend` _returnvalue (`/Game/Blueprints/MenuCameras_BP.CameraStart` _returnvalue_3) 0.0 "VTBlend_Cubic" 1.0 false)
      (`PlayerController.SetViewTargetWithBlend` _returnvalue (`/Game/Blueprints/MenuCameras_BP.CameraEnd` _returnvalue_3) _menucameratransitiontime "VTBlend_EaseInOut" 1.0 false)
      (`KismetSystemLibrary.Delay` (+ _menucameratransitiontime 0.0))
      (`/Game/Blueprints/MenuCameras_BP.StartRotation` _returnvalue_3))
    (:`Is Not Valid`
      _))
  (bind _asgj_hud (cast `/Game/Blueprints/Menus/GJ_HUD` (`PlayerController.GetHUD` (`GameplayStatics.GetPlayerController` 0))))
  (`/Game/Blueprints/Menus/GJ_HUD.ShowMainMenuhud` _asgj_hud))

(event `self.ReceiveTick`
  (params (DeltaSeconds :type "Float (single-precision)"))
  (if (and (<= (`self.CurrentGameTime`) 20) (`self.MusicOn`) (`self.GameIsPlaying`))
    (`/Engine/EditorBlueprintResources/StandardMacros.DoOnce` false
      (:`Completed`
        (`AudioComponent.FadeOut` (`self.CurrentMusic`) 2.0 0.0)
        (bind _returnvalue (`GameplayStatics.SpawnSound2D` "/Game/Audio/Music/DangerMusic_Cue.DangerMusic_Cue" 1.0 1.0 0.0 null))
        (bind _output_get (set `self.CurrentMusic` _returnvalue))
        (`AudioComponent.FadeIn` _output_get 2.0 1.0 0.0)))))

(event `StartGame`
  (params (multiplayer :type Boolean))
  (`self.ShowGameUI`)
  (`self.SpawnPlayers` multiplayer)
  (`self.StartTimer`)
  (if (`self.MusicOn`)
    (`AudioComponent.Stop` (`self.CurrentMusic`))
    (bind _returnvalue (`GameplayStatics.SpawnSound2D` "/Game/Audio/Music/Alien_Cue.Alien_Cue" 1.0 1.0 0.0 null))
    (set `self.CurrentMusic` _returnvalue)
    (set `self.GameIsPlaying` true)))

(fn `AddAlienPoints`
  (params (delta :type Integer))
  (set `self.AlienPoints` (+ (`KismetMathLibrary.Round` (* delta (`self.HumanPointMultiplier`))) (`self.AlienPoints`)))
  (`self.CheckMaxPointsReached`)
  (`GameplayStatics.PlaySound2D` "/Game/Audio/SFX/AlienSaying_Cue.AlienSaying_Cue" 1.0 1.0 0.0 null null))

(fn `AddHumanToAlien`
  (params (HumanPointValue :type Integer))
  (`self.AddAlienPoints` HumanPointValue))

(fn `AddHumanToReptile`
  (params (HumanPointValue :type Integer))
  (`self.AddReptilePoints` HumanPointValue))

(fn `AddReptilePoints`
  (params (delta :type Integer))
  (set `self.ReptilePoints` (+ (`KismetMathLibrary.Round` (* delta (`self.HumanPointMultiplier`))) (`self.ReptilePoints`)))
  (`self.CheckMaxPointsReached`)
  (`GameplayStatics.PlaySound2D` "/Game/Audio/SFX/ReptileSlither_Cue.ReptileSlither_Cue" 1.0 1.0 0.0 null null))

(fn `CheckMaxPointsReached`
  (if (> (`self.AlienPoints`) (`self.PointsToWin`))
    (`self.GameOver` :!label _label)
    (elif (> (`self.ReptilePoints`) (`self.PointsToWin`))
      (goto _label))))

(fn `CheckWeightedSums`
  (if (!= (+ (`self.PercentSpawn_Adult`) (`self.PercentSpawn_Elderly`) (`self.PercentSpawn_Child`) (`self.PercentSpawn_Teenager`)) 100)
    (`KismetSystemLibrary.PrintString` "SpawnWeightSums is not 100!!!" true true (struct :`G` 0.66 :`B` 1.0 :`A` 1.0) 5.0)))

(fn `DecreaseTime`
  (bind _result (`/Engine/EditorBlueprintResources/StandardMacros.DecrementInt` (`self.CurrentGameTime`))
    (:`  `
      (if (<= _result 0)
        (`KismetSystemLibrary.K2_ClearTimer` self "DecreaseTime")
        (`self.GameOver`)))))

(fn `GameOver`
  (locals (winner :type Integer))
  (bind _alienpoints (`self.AlienPoints`))
  (bind _reptilepoints (`self.ReptilePoints`))
  (if (`self.GameOverEnabled`)
    (bind _outactors (`GameplayStatics.GetAllActorsOfClass` "/Game/Blueprints/GJ_PlayerCharacter.GJ_PlayerCharacter_C"))
    (for _array_element _outactors
      (`self.DisableInput` _array_element (`GameplayStatics.GetPlayerController` 0))
      (set `self.isGameOver` true)
      (bind _asgj_hud (cast `/Game/Blueprints/Menus/GJ_HUD` (`PlayerController.GetHUD` (`GameplayStatics.GetPlayerController` 0))))
      (if (> _alienpoints _reptilepoints)
        (set `local.winner` 1)
        (elif (!= _alienpoints _reptilepoints)
          (set `local.winner` 2)))
      (`/Game/Blueprints/Menus/GJ_HUD.ShowEndGameUI` _asgj_hud (`local.winner`)))))

(fn `GetWeightedSpawnInt`
  (returns (humanTypeInt :type Integer))
  (locals (RandomInt :type Integer) (Sum :type Integer) (typeInt :type Integer))
  (bind _percentspawn_adult (`self.PercentSpawn_Adult`))
  (bind _output_get (set `local.RandomInt` (`KismetMathLibrary.RandomIntegerInRange` 0 99)))
  ;[1 1 1] Adult
  (if (< _output_get _percentspawn_adult)
    (return 0)
    (else
      (set `local.Sum` (+ (`local.Sum`) _percentspawn_adult))
      ;[1 1 1] Elderly
      (if (< (`local.RandomInt`) (+ (`self.PercentSpawn_Elderly`) (`local.Sum`)))
        (return 1)
        (else
          (set `local.Sum` (+ (`local.Sum`) (`self.PercentSpawn_Elderly`)))
          ;[1 1 1] Child
          (if (< (`local.RandomInt`) (+ (`self.PercentSpawn_Child`) (`local.Sum`)))
            (return 2)
            (else
              (set `local.Sum` (+ (`local.Sum`) (`self.PercentSpawn_Child`)))
              ;[1 1 1] Teenager
              (if (< (`local.RandomInt`) (+ (`self.PercentSpawn_Teenager`) (`local.Sum`)))
                (return 3)
                (else
                  (set `local.Sum` (+ (`local.Sum`) (`self.PercentSpawn_Teenager`)))
                  (return 0))))))))))

(fn `ShowGameUI`
  (bind _asgj_hud (cast `/Game/Blueprints/Menus/GJ_HUD` (`PlayerController.GetHUD` (`GameplayStatics.GetPlayerController` 0))))
  (`/Game/Blueprints/Menus/GJ_HUD.ShowGameUIhud` _asgj_hud))

(fn `ShowMainMenu`
  (bind _returnvalue (`GameplayStatics.GetPlayerController` 0))
  (`WidgetLayoutLibrary.RemoveAllWidgets`)
  (`/Engine/EditorBlueprintResources/StandardMacros.IsValid` (`self.m_MainMenu`)
    (:`Is Valid`
      _)
    (:`Is Not Valid`
      (bind _returnvalue_2 (`|CreateWidget` "/Game/Blueprints/Menus/GJ_MainMenu.GJ_MainMenu_C"))
      (set `self.m_MainMenu` _returnvalue_2)))
  (`UserWidget.AddToViewport` (`self.m_MainMenu`) 0)
  (`WidgetBlueprintLibrary.SetInputMode_UIOnlyEx` _returnvalue (`self.m_MainMenu`))
  (set `PlayerController.bShowMouseCursor` true _returnvalue))

(fn `SpawnHumans`
  (locals (numAdults :type Integer) (numElderly :type Integer) (numChilds :type Integer) (numTeens :type Integer))
  (bind _spawnpointarray (`self.SpawnPointArray`))
  (bind _spawnpointarray_2 (`self.SpawnPointArray`))
  ;[1 1 1] Makes Array Of All Spawn Locations
  (bind _outactors (`GameplayStatics.GetAllActorsOfClass` "/Game/Blueprints/SpawnPOints/NPCSpawnPoint.NPCSpawnPoint_C"))
  (for _array_element _outactors
    (`KismetArrayLibrary.Array_Add` _spawnpointarray _array_element))
  (`KismetSystemLibrary.PrintString` (`KismetTextLibrary.Conv_TextToString` (`|FormatText` "There are {0} spawn points" (`KismetArrayLibrary.Array_Length` _spawnpointarray))) true true (struct :`G` 0.66 :`B` 1.0 :`A` 1.0) 5.0)
  (`self.CheckWeightedSums`)
  (`KismetArrayLibrary.Array_Shuffle` _spawnpointarray_2)
  (for (_array_element_2 _array_index) _spawnpointarray_2
    (if (< (/ (`KismetMathLibrary.Conv_IntToDouble` _array_index) (`KismetMathLibrary.Conv_IntToDouble` (`KismetArrayLibrary.Array_Length` _spawnpointarray_2))) (/ (`self.PercentageOfSpawnsUsed`) 100.0))
      (bind _humantypeint (`self.GetWeightedSpawnInt`))
      (switch `int` _humantypeint
        (:`0`
          (bind _returnvalue (`self.GetTransform` _array_element_2))
          ;[1 1 1] Spawning NPC Adults
          (`|SpawnActorFromClass` "/Game/Blueprints/NPC_Human_BP_Children/Human_Adult.Human_Adult_C" _returnvalue "Undefined" "OverrideRootScale" null null)
          (`/Engine/EditorBlueprintResources/StandardMacros.IncrementInt` (`local.numAdults`)))
        (:`1`
          ;[1 1 1] Spawning NPC Elders
          (`|SpawnActorFromClass` "/Game/Blueprints/NPC_Human_BP_Children/Human_Elder.Human_Elder_C" _returnvalue "Undefined" "OverrideRootScale" null null)
          (`/Engine/EditorBlueprintResources/StandardMacros.IncrementInt` (`local.numElderly`)))
        (:`2`
          ;[1 1 1] Spawning NPC Childs
          (`|SpawnActorFromClass` "/Game/Blueprints/NPC_Human_BP_Children/Human_Child.Human_Child_C" _returnvalue "Undefined" "OverrideRootScale" null null)
          (`/Engine/EditorBlueprintResources/StandardMacros.IncrementInt` (`local.numChilds`)))
        (:`3`
          ;[1 1 1] Spawning NPC Conspirators
          (`|SpawnActorFromClass` "/Game/Blueprints/NPC_Human_BP_Children/Human_Conspiracy_Theorist.Human_Conspiracy_Theorist_C" _returnvalue "Undefined" "OverrideRootScale" null null)
          (`/Engine/EditorBlueprintResources/StandardMacros.IncrementInt` (`local.numTeens`))))
      (else
        (`KismetSystemLibrary.PrintString` (`KismetTextLibrary.Conv_TextToString` (`|FormatText` "Spawned {0} humans" _array_index)) true true (struct :`G` 0.66 :`B` 1.0 :`A` 1.0) 5.0)
        (break))))
  (`KismetSystemLibrary.PrintString` (`KismetTextLibrary.Conv_TextToString` (`|FormatText` "Spawned {0} adults" (`local.numAdults`))) true true (struct :`G` 0.66 :`B` 1.0 :`A` 1.0) 5.0)
  (`KismetSystemLibrary.PrintString` (`KismetTextLibrary.Conv_TextToString` (`|FormatText` "Spawned {0} elderly" (`local.numElderly`))) true true (struct :`G` 0.66 :`B` 1.0 :`A` 1.0) 5.0)
  (`KismetSystemLibrary.PrintString` (`KismetTextLibrary.Conv_TextToString` (`|FormatText` "Spawned {0} childs" (`local.numChilds`))) true true (struct :`G` 0.66 :`B` 1.0 :`A` 1.0) 5.0)
  (`KismetSystemLibrary.PrintString` (`KismetTextLibrary.Conv_TextToString` (`|FormatText` "Spawned {0} teens" (`local.numTeens`))) true true (struct :`G` 0.66 :`B` 1.0 :`A` 1.0) 5.0))

(fn `SpawnPlayers`
  (params (multiplayer :type Boolean))
  (set `self.Multiplayer` multiplayer)
  (bind _outactors (`GameplayStatics.GetAllActorsOfClass` "/Script/Engine.PlayerStart"))
  (for _array_element _outactors
    (if (== (`PlayerStart.PlayerStartTag` _array_element) "Reptile")
      (`GameplayStatics.CreatePlayer` 0)
      (bind _returnvalue (`self.GetTransform` _array_element))
      (bind _returnvalue_2 (`|SpawnActorFromClass` "/Game/Blueprints/GJ_PlayerCharacter.GJ_PlayerCharacter_C" _returnvalue "AlwaysSpawn" "OverrideRootScale" null false null))
      (`Controller.Possess` (`GameplayStatics.GetPlayerController` 0) _returnvalue_2)
      (if (not (`self.Multiplayer`))
        (`/Game/Blueprints/GJ_PlayerCharacter.RotateCameraAngle` _returnvalue_2))
      (elif (`self.Multiplayer`)
        (`GameplayStatics.CreatePlayer` 1)
        (bind _returnvalue_3 (`|SpawnActorFromClass` "/Game/Blueprints/GJ_PlayerCharacter.GJ_PlayerCharacter_C" _returnvalue "AlwaysSpawn" "OverrideRootScale" null true null))
        (`Controller.Possess` (`GameplayStatics.GetPlayerController` 1) _returnvalue_3)))))

(fn `StartTimer`
  (set `self.CurrentGameTime` (`self.TotalGameTime`))
  (`KismetSystemLibrary.K2_SetTimer` null "DecreaseTime" 1.0 true))

(fn `UserConstructionScript`)