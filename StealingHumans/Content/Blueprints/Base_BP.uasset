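; Base_BP is a base actor that tracks the humans placed inside it, likely as a parent for team or player bases.
; AddHumanToBase adds a human to HumansInBase only once and passes its point value and dragged flag to AddHumanPoints, an empty hook for scoring.
; PrisonBreak loops over every held human and calls BreakOutOfBase on each.
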(fn `AddHumanPoints`
  (params (HumanPointValue :type Integer) (dragged :type Boolean)))

(fn `AddHumanToBase`
  (params (Human :type "/Game/Blueprints/NPC_Human Object Reference") (dragged :type Boolean))
  (if (not (`KismetArrayLibrary.Array_Contains` (`self.HumansInBase`) Human))
    (`KismetArrayLibrary.Array_Add` (`self.HumansInBase`) Human)
    (`self.AddHumanPoints` (`/Game/Blueprints/NPC_Human.PointValue` Human) dragged)))

(fn `PrisonBreak`
  (for _array_element (`self.HumansInBase`)
    (`/Game/Blueprints/NPC_Human.BreakOutOfBase` _array_element)))

(fn `UserConstructionScript`)