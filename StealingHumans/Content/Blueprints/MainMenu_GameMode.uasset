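; MainMenu_GameMode is a game mode that keeps Alien and Reptile team scores and a match countdown.
; Human capture functions add point values to either side, and each addition checks whether a score exceeds PointsToWin.
; A looping one-second timer started on BeginPlay decrements TotalGameTime.
; Time-out or a winning score calls GameOver, which is empty; its input-disabling and HUD logic is disconnected.
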(event `self.ReceiveBeginPlay`
  (`self.StartTimer`))

(fn `AddAlienPoints`
  (params (delta :type Integer))
  (set `self.AlienPoints` (+ delta (`self.AlienPoints`)))
  (`self.CheckMaxPointsReached`))

(fn `AddHumanToAlien`
  (params (HumanPointValue :type Integer))
  (`self.AddAlienPoints` HumanPointValue))

(fn `AddHumanToReptile`
  (params (HumanPointValue :type Integer))
  (`self.AddReptilePoints` HumanPointValue))

(fn `AddReptilePoints`
  (params (delta :type Integer))
  (set `self.ReptilePoints` (+ delta (`self.ReptilePoints`)))
  (`self.CheckMaxPointsReached`))

(fn `CheckMaxPointsReached`
  (if (> (`self.AlienPoints`) (`self.PointsToWin`))
    (`self.GameOver` :!label _label)
    (elif (> (`self.ReptilePoints`) (`self.PointsToWin`))
      (goto _label))))

(fn `DecreaseTime`
  (bind _result (`/Engine/EditorBlueprintResources/StandardMacros.DecrementInt` (`self.TotalGameTime`))
    (:`  `
      (if (<= _result 0)
        (`KismetSystemLibrary.K2_ClearTimer` self "DecreaseTime")
        (`self.GameOver`)))))

(fn `GameOver`)

(fn `StartTimer`
  (`KismetSystemLibrary.K2_SetTimer` null "DecreaseTime" 1.0 true))

(fn `UserConstructionScript`)